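; BP_ItemMaster is a base pickup actor for inventory items in the world.
; On BeginPlay it fills a missing ItemObject through GetDefaultItemObject, which returns nothing here, apparently a hook for child Blueprints to override.
; When a ThirdPersonCharacter overlaps its Collision, it passes the item to that character's BPInventoryComponent via TryAddItem and destroys itself only if the add succeeds.
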(event `self.ReceiveBeginPlay`
  (`/Engine/EditorBlueprintResources/StandardMacros.IsValid` (`self.ItemObject`)
    (:`Is Not Valid`
      (set `self.ItemObject` (`self.GetDefaultItemObject`)))))

(event `self.Collision.OnComponentBeginOverlap`
  (params (OverlappedComponent :type "PrimitiveComponent Object Reference") (OtherActor :type "Actor Object Reference") (OtherComp :type "PrimitiveComponent Object Reference") (OtherBodyIndex :type Integer) (bFromSweep :type Boolean) (SweepResult :type "HitResult Structure (by ref)"))
  (bind _asthird_person_character (cast `/Game/ThirdPersonBP/Blueprints/ThirdPersonCharacter` OtherActor))
  (bind _success (`/Game/Inventory/BP_InventoryComponent.TryAddItem` (`/Game/ThirdPersonBP/Blueprints/ThirdPersonCharacter.BP_InventoryComponent` _asthird_person_character) (`self.ItemObject`)))
  (if _success
    (`self.K2_DestroyActor`)))

(fn `GetDefaultItemObject`
  (returns (ItemObject :type "/Game/Inventory/ItemActors/BP_ItemObject Object Reference"))
  (return null))

(fn `UserConstructionScript`)