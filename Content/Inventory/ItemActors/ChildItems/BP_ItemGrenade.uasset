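; BP_ItemGrenade is a child item actor that represents a grenade in the inventory system.
; It overrides GetDefaultItemObject to construct a BP_ItemObject using the actor's ItemDimensions, normal and rotated grenade icon materials, and its own class as ItemClass.
; The event graph holds only disabled stubs, and the construction script just calls the parent, so the file adds no other behavior.
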(fn `GetDefaultItemObject`
  (returns (ItemObject :type "/Game/Inventory/ItemActors/BP_ItemObject Object Reference"))
  (bind _returnvalue (`|GenericCreateObject` "/Game/Inventory/ItemActors/BP_ItemObject.BP_ItemObject_C" self (`self.ItemDimensions`) "/Game/Inventory/Textures/Icons/MI_Grenade.MI_Grenade" "/Game/Inventory/Textures/Icons/MI_Grenade_Rotated.MI_Grenade_Rotated" "BP_ItemGrenade_C"))
  (return _returnvalue))

(fn `UserConstructionScript`
  (`parent.UserConstructionScript`))