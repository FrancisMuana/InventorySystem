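; Inventory component that stores multi-tile items in a Columns by Rows grid, backed by a flat array of item references.
; TryAddItem takes the first spot where the item's footprint fits, retrying with the item rotated if none is free.
; Macros walk and bounds-check footprints; GetAllItems maps each unique item to its top-left tile.
; Adds and removals set a dirty flag, so Tick broadcasts the inventory change.
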(event `self.ReceiveBeginPlay`
  (`KismetArrayLibrary.Array_Resize` (`self.Items`) (* (`self.Columns`) (`self.Rows`))))

(event `self.ReceiveTick`
  (params (DeltaSeconds :type "Float (single-precision)"))
  (if (`self.IsDirty`)
    (set `self.IsDirty` false)
    (`self.OnInventoryChanged`)))

(fn `AddItemAt`
  (params (ItemObject :type "/Game/Inventory/ItemActors/BP_ItemObject Object Reference") (TopLeftIndex :type Integer))
  (bind _tile (`self.ForEachIndex` ItemObject TopLeftIndex)
    (:`LoopBody`
      (`KismetArrayLibrary.Array_Set` (`self.Items`) (`self.TileToIndex` _tile) (`local.ItemObject`)))
    (:`Completed`
      (set `self.IsDirty` true))))

(fn `GetAllItems`
  (returns (AllItems :type "Map of /Game/Inventory/ItemActors/BP_ItemObject Object Reference to /Game/Inventory/Structs/S_Tile Structure"))
  (locals (LocalAllItems :type "Map of /Game/Inventory/ItemActors/BP_ItemObject Object Reference to /Game/Inventory/Structs/S_Tile Structure") (LocalItemObject :type "/Game/Inventory/ItemActors/BP_ItemObject Object Reference") (LocalIndex :type Integer))
  (for (_array_element _array_index) (`self.Items`)
    (bind _output_get (set `local.LocalItemObject` _array_element))
    (`/Engine/EditorBlueprintResources/StandardMacros.IsValid` _output_get
      (:`Is Valid`
        (set `local.LocalIndex` _array_index)
        (if (not (`BlueprintMapLibrary.Map_Contains` (`local.LocalAllItems`) (`local.LocalItemObject`)))
          (`BlueprintMapLibrary.Map_Add` (`local.LocalAllItems`) (`local.LocalItemObject`) (`self.IndexToTile` (`local.LocalIndex`)))))))
  (return (`local.LocalAllItems`)))

(fn `GetItemAtIndex`
  (params (Index :type Integer))
  (returns (Success :type Boolean) (ItemObject :type "/Game/Inventory/ItemActors/BP_ItemObject Object Reference"))
  (locals (LocalIndex :type Integer))
  (set `local.LocalIndex` Index)
  (if (`KismetArrayLibrary.Array_IsValidIndex` (`self.Items`) (`local.LocalIndex`))
    (return true (`|GetArrayItem` (`self.Items`) (`local.LocalIndex`)))
    (else
      (return false null))))

(fn `IndexToTile`
  (params (Index :type Integer))
  (returns (Tile :type "/Game/Inventory/Structs/S_Tile Structure"))
  (locals (LocalTile :type "/Game/Inventory/Structs/S_Tile Structure"))
  (set `local.LocalTile` (make `/Game/Inventory/Structs/S_Tile` (mod Index (`self.Columns`)) (/ Index (`self.Columns`))))
  (return (`local.LocalTile`)))

(fn `IsSpaceAvailable`
  (params (ItemObject :type "/Game/Inventory/ItemActors/BP_ItemObject Object Reference") (TopLeftIndex :type Integer))
  (returns (Success :type Boolean))
  (`|ExecutionSequence`
    (:`then_0`
      (bind _tile (`self.ForEachIndex` ItemObject TopLeftIndex)
        (:`LoopBody`
          (`self.IsTileValid` _tile
            (:`true`
              (bind (_success _itemobject) (`self.GetItemAtIndex` (`self.TileToIndex` _tile)))
              (if _success
                (if (`KismetSystemLibrary.IsValid` _itemobject)
                  (return false))
                (else
                  (return false))))
            (:`false`
              (return false))))))
    (:`then_1`
      (return true))))

(fn `RemoveItemFromInventory`
  (params (ItemObject :type "/Game/Inventory/ItemActors/BP_ItemObject Object Reference"))
  (`/Engine/EditorBlueprintResources/StandardMacros.IsValid` ItemObject
    (:`Is Valid`
      (for (_array_element _array_index) (`self.Items`)
        (if (== _array_element (`local.ItemObject`))
          (`KismetArrayLibrary.Array_Set` (`self.Items`) _array_index)
          (set `self.IsDirty` true))))))

(fn `TileToIndex`
  (params (Tile :type "/Game/Inventory/Structs/S_Tile Structure"))
  (returns (Index :type Integer))
  (bind (_x _y) (break `/Game/Inventory/Structs/S_Tile` Tile))
  (return (+ _x (* _y (`self.Columns`)))))

(fn `TryAddItem`
  (params (ItemObject :type "/Game/Inventory/ItemActors/BP_ItemObject Object Reference"))
  (returns (Success :type Boolean))
  (`/Engine/EditorBlueprintResources/StandardMacros.IsValid` ItemObject
    (:`Is Valid`
      (for (_ _array_index) (`self.Items`) :!label _label
        (bind _success (`self.IsSpaceAvailable` (`local.ItemObject`) _array_index))
        (if _success
          (`self.AddItemAt` (`local.ItemObject`) _array_index)
          (return true)))
      (`|ExecutionSequence`
        (:`then_0`
          (`/Engine/EditorBlueprintResources/StandardMacros.DoOnce` false
            (:`Completed`
              (`/Game/Inventory/ItemActors/BP_ItemObject.Rotate` (`local.ItemObject`))
              (goto _label))))
        (:`then_1`
          (`/Game/Inventory/ItemActors/BP_ItemObject.Rotate` (`local.ItemObject`))
          (return false))))))