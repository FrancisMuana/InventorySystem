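; Game State Blueprint for the inventory system that provides a function to spawn an item object back into the world as an actor.
; SpawnItemFromActor places the spawn point a short distance in front of the owning actor, optionally snapping it to a surface found by a downward-angled Visibility trace.
; It then spawns the item's class there regardless of collision, passing the ItemObject to the new actor.
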(fn `SpawnItemFromActor`
  (params (ItemObject :type "/Game/Inventory/ItemActors/BP_ItemObject Object Reference") (OwningActor :type "Actor Object Reference") (GroundClamp :type Boolean))
  (locals (LocalSpawnLocation :type "Vector Structure"))
  (bind _itemobject (`local.ItemObject`))
  (bind _owningactor (`local.OwningActor`))
  (`|ExecutionSequence`
    (:`then_0`
      (set `local.LocalSpawnLocation` (+ (`self.K2_GetActorLocation` _owningactor) (* (`self.GetActorForwardVector` _owningactor) 150.0)))
      (if (`local.GroundClamp`)
        (bind (_outhit _returnvalue) (`KismetSystemLibrary.LineTraceSingle` (`self.K2_GetActorLocation` (`local.OwningActor`)) (- (`local.LocalSpawnLocation`) (0.0 0.0 100.0)) "TraceTypeQuery1"))
        (if _returnvalue
          (set `local.LocalSpawnLocation` (`.Location` (`GameplayStatics.BreakHitResult` _outhit))))))
    (:`then_1`
      (`|SpawnActorFromClass` (`/Game/Inventory/ItemActors/BP_ItemObject.GetItemClass` _itemobject) (`KismetMathLibrary.MakeTransform` (`local.LocalSpawnLocation`) (struct)) "AlwaysSpawn" "OverrideRootScale" null _itemobject null))))

(fn `UserConstructionScript`)